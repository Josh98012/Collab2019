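; Base Blueprint for side objectives in the objective system, handling a step's tag and trigger box.
; ProgressMission optionally spawns the CurrentSubObjective actor at its own transform as the tag, and enables the trigger box with a self reference when a collision box is flagged.
; DestroySelf destroys the trigger box and tag, then calls CallCompleted to signal completion.
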(event Custom|ProgressMission
  (if (Variables|Default|GetShowTag?)
    (bind _returnvalue (Game|SpawnActorfromClass "/Game/Users/Dawid/TestBlueprints/ObjectiveSystem/CurrentSubObjective.CurrentSubObjective_C" (Transformation|GetActorTransform) "Undefined" 0 0))
    (Variables|Default|SetSubObjTag _returnvalue))
  (if (Variables|Default|GetHasACollisionBox)
    (Default|EnableMission (Variables|Default|GetTriggerBox) self)))

(event Custom|DestroySelf
  (Actor|DestroyActor (Variables|Default|GetTriggerBox))
  (Actor|DestroyActor (Variables|Default|GetSubObjTag))
  (Default|CallCompleted))

(fn ConstructionScript)