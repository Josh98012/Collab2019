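; Oil barrel trap that leaks oil when something overlaps it and can set the spilled oil on fire.
; Barrel overlaps spawn a water particle emitter as the leak, whose particle collisions place short-lived decals and, after a delay, collision actors tracked briefly in an array.
; Overlapping a collision actor stops further leaks, destroys the emitters and spawns fire effects at every tracked oil spot.
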(event OnComponentBeginOverlap(Barrel)
  (params (OverlappedComponent :type Primitive%20Component%20Object%20Reference) (OtherActor :type Actor%20Object%20Reference) (OtherComp :type Primitive%20Component%20Object%20Reference) (OtherBodyIndex :type Integer) (bFromSweep :type Boolean) (SweepResult :type Hit%20Result%20Structure%20%28by%20ref%29))
  ;[1 1 1] Damage system
  (if (Variables|Default|GetCanBeDamaged)
    (bind _returnvalue (Effects|SpawnEmitteratLocation "/Game/Users/Dawid/TestBlueprints/Particles/PAR_Water_CPU.PAR_Water_CPU" (.impactpoint SweepResult) (* (Transformation|GetActorRotation OtherActor) -1.0)))
    (Utilities|Array|Add (Variables|Default|GetOilEmmiters) _returnvalue)
    (EventDispatchers|BindEventtoOnParticleCollide _returnvalue (delegate Custom|Collided))))

(event Custom|Collided
  (params (EventName :type Name) (EmitterTime :type Float%20%28single-precision%29) (ParticleTime :type Integer) (Location :type Vector) (Velocity :type Vector) (Direction :type Vector) (Normal :type Vector) (BoneName :type Name) (PhysMat :type Physical%20Material%20Object%20Reference))
  (bind _returnvalue (Math|Conversions|RotationFromXVector Normal))
  (bind _oilcollision (Variables|Default|GetOilCollision))
  (bind _returnvalue_2 (Rendering|Material|CreateDynamicMaterialInstance "/Engine/MapTemplates/Materials/BasicAsset01.BasicAsset01" "None" :!class /Script/Engine.KismetMaterialLibrary))
  (Rendering|Decal|SpawnDecalatLocation _returnvalue_2 (Math|Conversions|ToVector(Float) (Math|Random|RandomFloatinRange 2e+01 5e+01)) Location _returnvalue 2.5)
  (Utilities|FlowControl|Delay 2.0)
  (bind _returnvalue_3 (Game|SpawnActorfromClass "/Game/Users/Dawid/TestBlueprints/Traps/OilCollision.OilCollision_C" (Math|Transform|MakeTransform Location _returnvalue "1,1,1") "Undefined" 0 0))
  (Utilities|Array|Add _oilcollision _returnvalue_3)
  (Collision|BindEventtoOnActorBeginOverlap _returnvalue_3 (delegate Custom|Overlapped))
  (Utilities|FlowControl|Delay 1.0)
  (Utilities|Array|RemoveItem _oilcollision _returnvalue_3))

(event Custom|Overlapped
  (params (OverlappedActor :type Actor%20Object%20Reference) (OtherActor :type Actor%20Object%20Reference))
  (Variables|Default|SetCanBeDamaged false)
  (for _array_element (Variables|Default|GetOilEmmiters)
    (Components|DestroyComponent _array_element))
  (for _array_element_2 (Variables|Default|GetOilCollision)
    (Effects|SpawnEmitteratLocation "/Game/StarterContent/Particles/P_Fire.P_Fire" (Transformation|GetWorldLocation (Variables|/Script/Engine.Actor|GetRootComponent _array_element_2)) (Math|Conversions|RotationFromXVector (stale Custom|Collided Normal)) "2.000000,2.000000,2.000000")))

(fn ConstructionScript)