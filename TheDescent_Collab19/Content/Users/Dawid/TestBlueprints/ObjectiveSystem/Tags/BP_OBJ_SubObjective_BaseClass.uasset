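; Base sub-objective actor for an objective system, with an optional tag actor that marks it in the world.
; On BeginPlay, if HasATag is set, it spawns the CurrentSubObjective class at its root transform and stores it as Tag.
; SubObjectiveCompleted flags completion and calls CallSubCompleted, then destroys the tag.
; Without a tag, it destroys itself instead if DestroyOnComplete is set.
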(event Custom|SubObjectiveCompleted
  ;[1 1 1] On objective complete, destroy tag and actor if required
  (Variables|Default|SetCompleted true)
  (Default|CallSubCompleted)
  (if (Variables|Default|GetHasATag?)
    (Actor|DestroyActor (Variables|Default|GetTag))
    (elif (Variables|Default|GetDestroyOnComplete?)
      (Actor|DestroyActor))))

(event EventBeginPlay
  ;[1 1 1] On being play spawn sub objective
  (if (Variables|Default|GetHasATag?)
    (bind _returnvalue (Game|SpawnActorfromClass "/Game/Users/Dawid/TestBlueprints/ObjectiveSystem/CurrentSubObjective.CurrentSubObjective_C" (Transformation|GetWorldTransform (Variables|Default|GetDefaultSceneRoot)) "Undefined" 0 0))
    (Variables|Default|SetTag _returnvalue)))

(fn ConstructionScript)