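; BP_OBJ_FindWife_Tag is a main objective in a tag-based objective system, apparently for finding the wife.
; On BeginPlay it registers itself with every CurrentObejctive actor as the new objective and sends info to the widget.
; When it has a collision box, it binds to each side objective's completion event.
; A counter tallies completed side objectives and enables the TriggerBox collision once all are done.
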(event Custom|CheckIfObjCompleted
  (bind _result (Math|Integer|IncrementInt (Variables|Default|GetTempNum001))
    (:%20%20
      (if (== _result (Utilities|Array|Length (Variables|Default|GetSideObjectives)))
        (Default|EnableCollision (Variables|Default|GetTriggerBox))))))

(event EventBeginPlay
  (bind _outactors (Actor|GetAllActorsOfClass "/Game/Users/Dawid/TestBlueprints/ObjectiveSystem/CurrentObejctive.CurrentObejctive_C"))
  (for _array_element _outactors
    (Class|INTObjectives|StartNewObjective(Message) _array_element self))
  (Class|INTObjectives|SendInfotoWidget(Message) _array_element "NewEnumerator8")
  (if (Variables|Default|GetHasACollisionBox)
    (for _array_element_2 (Variables|Default|GetSideObjectives)
      (EventDispatchers|BindEventtoSubCompleted _array_element_2 (delegate Custom|CheckIfObjCompleted)))))

(fn ConstructionScript)