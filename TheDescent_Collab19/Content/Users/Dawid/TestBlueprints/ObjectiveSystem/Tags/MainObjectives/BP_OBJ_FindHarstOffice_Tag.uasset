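; Main objective tag for finding Harst's office that tracks side objective items and tags through completion events and counters.
; StartNewObjective binds items if it has a collision box; otherwise it binds and progresses tags, updates objective actors, and enables TriggerBox if no sub-objectives are needed.
; Item completion enables TriggerBox once the required sets are done.
; Completing all tags only sets their flag and destroys them, without rechecking the trigger.
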(event Custom|SubCompleted
  (bind _sideobjectivetags (Variables|Default|GetSideObjectiveTags))
  ;[1 1 1] Check if all sub objectives are completed
  (bind _result (Math|Integer|IncrementInt (Variables|Default|GetTempNum002))
    (:%20%20
      (if (== _result (Utilities|Array|Length _sideobjectivetags))
        (Variables|Default|SetSOTCompleted true)
        ;[1 1 1] Destroy the tags
        (for _array_element _sideobjectivetags
          (Actor|DestroyActor _array_element))))))

(event Custom|CheckIfObjCompleted
  (bind _result (Math|Integer|IncrementInt (Variables|Default|GetTempNum001))
    (:%20%20
      (if (== _result (Utilities|Array|Length (Variables|Default|GetSideObjectives)))
        (Variables|Default|SetSOICompleted true)
        ;[1 1 1] Check the appropriate arrays and see if objectives are completed
        (if (and (Variables|Default|GetHasSubObjectiveItems) (Variables|Default|GetHasSubObjectiveTags))
          (if (and (Variables|Default|GetSOICompleted) (Variables|Default|GetSOTCompleted))
            (Default|EnableCollision (Variables|Default|GetTriggerBox) :!label _label))
          (elif (Variables|Default|GetHasSubObjectiveItems)
            (if (Variables|Default|GetSOICompleted)
              (goto _label))
            (elif (Variables|Default|GetHasSubObjectiveTags)
              (if (Variables|Default|GetSOTCompleted)
                (goto _label)))))))))

(event Custom|DestroyTags
  ;[1 1 1] Destroy the tags
  (for _array_element (Variables|Default|GetSideObjectiveTags)
    (Actor|DestroyActor _array_element)))

(event EventStartNewObjective
  (params (NewTag :type BP%20OBJ%20Base%20Object%20Reference))
  (if (Variables|Default|GetHasACollisionBox)
    (for _array_element (Variables|Default|GetSideObjectives)
      (EventDispatchers|BindEventtoSubCompleted _array_element (delegate Custom|CheckIfObjCompleted)))
    ;[1 1 1] If there are more than 0 side objectives, set the bool to true
    (if (>= (Utilities|Array|Length (Variables|Default|GetSideObjectives)) 1)
      (Variables|Default|SetHasSubObjectiveItems true))
    (else
      (for _array_element_2 (Variables|Default|GetSideObjectiveTags)
        ;[1 1 1] Check if all sub objectives are completed
        (EventDispatchers|BindEventtoCompleted _array_element_2 (delegate Custom|SubCompleted)))
      (if (>= (Utilities|Array|Length (Variables|Default|GetSideObjectiveTags)) 1)
        (Variables|Default|SetHasSubObjectiveTags true))
      ;[1 1 1] Get current objective and update it
      (bind _outactors (Actor|GetAllActorsOfClass "/Game/Users/Dawid/TestBlueprints/ObjectiveSystem/CurrentObejctive.CurrentObejctive_C"))
      (for _array_element_3 _outactors
        (Class|INTObjectives|StartNewObjective(Message) _array_element_3 NewTag)
        (Class|INTObjectives|SendInfotoWidget(Message) _array_element_3 (Variables|Default|GetCurrentObjective)))
      ;[1 1 1] Enable side objective tags and, if necessary enable the collision boxes
      (for _array_element_4 (Variables|Default|GetSideObjectiveTags)
        (Default|ProgressMission _array_element_4))
      (if (not (Variables|Default|GetDoesNeedSubObjCompleted?))
        (Default|EnableCollision (Variables|Default|GetTriggerBox))))))

(fn ConstructionScript)