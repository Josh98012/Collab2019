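; Base mission trigger actor that starts a new objective when the player character overlaps it.
; It ignores overlaps until EnableCollision sets MissionEnabled, which acts as a flag without changing actual collision.
; An overlapping NewDrSkeng_USE receives the objective message, then all CurrentObejctive actors receive the new tag and widget info.
; The trigger then destroys itself, making it single-use.
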(event Custom|EnableCollision
  ;[1 1 1] Enable the collision when necessary
  (Variables|Default|SetMissionEnabled true))

(event Collision|EventActorBeginOverlap
  (params (OtherActor :type Actor%20Object%20Reference))
  (bind _newtag (Variables|Default|GetNewTag))
  ;[1 1 1] On overlap see if the mission is enabled
  (if (Variables|Default|GetMissionEnabled)
    ;[1 1 1] Send the info to the tablet widget
    (bind _asnew_dr_skeng_use (Utilities|Casting|CastToNewDrSkeng_USE OtherActor))
    (Class|INTObjectives|StartObjective(Message) _asnew_dr_skeng_use (Variables|Default|GetNewObjective))
    (Class|INTObjectives|StartNewObjective(Message) _newtag _newtag)
    ;[1 1 1] Send info to current objective to start new objective and delete the trigger after finish
    (bind _outactors (Actor|GetAllActorsOfClass "/Game/Users/Dawid/TestBlueprints/ObjectiveSystem/CurrentObejctive.CurrentObejctive_C"))
    (for _array_element _outactors
      (Class|INTObjectives|StartNewObjective(Message) _array_element _newtag)
      (Class|INTObjectives|SendInfotoWidget(Message) _array_element (Variables|Default|GetNewObjective))
      (Variables|Default|SetMissionEnabled false))
    (Actor|DestroyActor)))

(fn ConstructionScript)