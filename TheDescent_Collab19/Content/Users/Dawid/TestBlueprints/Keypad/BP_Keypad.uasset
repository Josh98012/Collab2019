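; Keypad actor that shows a UI_Keypad widget when the player presses interact inside its box trigger.
; BeginPlay creates the hidden widget and binds to JerrysCharacter1's interact event.
; A FlipFlop alternates between showing it (if overlapping), which locks movement, shows the cursor and sets UI-only input, and hiding it, which restores movement and hides the cursor without resetting input mode.
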(event OnComponentBeginOverlap(Box)
  (params (OverlappedComponent :type Primitive%20Component%20Object%20Reference) (OtherActor :type Actor%20Object%20Reference) (OtherComp :type Primitive%20Component%20Object%20Reference) (OtherBodyIndex :type Integer) (bFromSweep :type Boolean) (SweepResult :type Hit%20Result%20Structure%20%28by%20ref%29))
  (Variables|Default|SetIsOverlaping true))

(event OnComponentEndOverlap(Box)
  (params (OverlappedComponent :type Primitive%20Component%20Object%20Reference) (OtherActor :type Actor%20Object%20Reference) (OtherComp :type Primitive%20Component%20Object%20Reference) (OtherBodyIndex :type Integer))
  (Variables|Default|SetIsOverlaping false))

(event Custom|Overlap
  (bind _ui_keypad_ref (Variables|Default|GetUI_Keypad_Ref))
  (bind _char_ref (Variables|Default|GetChar_Ref))
  (Utilities|FlowControl|FlipFlop
    (:A
      (if (Variables|Default|GetIsOverlaping)
        (Widget|SetVisibility _ui_keypad_ref "Visible")
        (Variables|/Game/Users/Jerry/Character/JerrysCharacter1.JerrysCharacter1_C|SetCanMove _char_ref false)
        (bind _asjerrys_character_controller (Utilities|Casting|CastToJerrysCharacterController (Pawn|GetController _char_ref)))
        (Variables|/Script/Engine.PlayerController|SetbShowMouseCursor _asjerrys_character_controller true)
        (Variables|Default|SetKeypadShown true)
        (Input|SetInputModeUIOnly _asjerrys_character_controller (Variables|Default|GetUI_Keypad_Ref) "DoNotLock")
        (else
          (Development|PrintString "Branch false"))))
    (:B
      (Widget|SetVisibility _ui_keypad_ref "Hidden")
      (Variables|/Game/Users/Jerry/Character/JerrysCharacter1.JerrysCharacter1_C|SetCanMove _char_ref true)
      (Variables|Default|SetKeypadShown false)
      (Variables|/Script/Engine.PlayerController|SetbShowMouseCursor _asjerrys_character_controller false))))

(event EventBeginPlay
  (bind _outactors (Actor|GetAllActorsOfClass "/Game/Users/Jerry/Character/JerrysCharacter1.JerrysCharacter1_C"))
  (for _array_element _outactors
    (bind _output_get (Variables|Default|SetChar_Ref _array_element))
    (bind _returnvalue (UserInterface|CreateWidget "/Game/Users/Dawid/TestBlueprints/Keypad/UI_Keypad.UI_Keypad_C" (Game|GetPlayerController 0)))
    (bind _output_get_2 (Variables|Default|SetUI_Keypad_Ref _returnvalue))
    (UserInterface|Viewport|AddtoPlayerScreen _output_get_2)
    (Widget|SetVisibility _output_get_2 "Hidden")
    (EventDispatchers|BindEventtoInteractButtonPressed _array_element (delegate Custom|Overlap))))

(fn ConstructionScript)