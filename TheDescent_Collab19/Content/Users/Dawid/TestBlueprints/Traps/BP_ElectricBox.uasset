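; BP_ElectricBox is a test trap: an electric box that electrocutes actors once it has been damaged.
; Any damage sets a Damaged flag and activates the Lightning component.
; While damaged, each overlap with ElectricutionRange applies one hit of configurable damage and type to the entering actor, then activates Lightning again after a short delay.
; The Damaged flag is never cleared in these graphs.
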(event OnComponentBeginOverlap(ElectricutionRange)
  (params (OverlappedComponent :type Primitive%20Component%20Object%20Reference) (OtherActor :type Actor%20Object%20Reference) (OtherComp :type Primitive%20Component%20Object%20Reference) (OtherBodyIndex :type Integer) (bFromSweep :type Boolean) (SweepResult :type Hit%20Result%20Structure%20%28by%20ref%29))
  (if (Variables|Default|GetDamaged)
    (Game|Damage|ApplyDamage OtherActor (Variables|Default|GetDamageOutput) 0 0 "/Script/Engine.DamageType")
    (Utilities|FlowControl|Delay 0.5)
    (Components|Activation|Activate (Variables|Default|GetLightning) false)))

(event Game|Damage|EventAnyDamage
  (params (Damage :type Float%20%28single-precision%29) (DamageType :type Damage%20Type%20Object%20Reference) (InstigatedBy :type Controller%20Object%20Reference) (DamageCauser :type Actor%20Object%20Reference))
  (Variables|Default|SetDamaged true)
  (Components|Activation|Activate (Variables|Default|GetLightning) false))

(fn ConstructionScript)