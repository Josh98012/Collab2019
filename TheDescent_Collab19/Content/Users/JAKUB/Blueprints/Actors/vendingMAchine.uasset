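; Vending machine actor prototype that lets a player pick one of three items and prints its cost.
; Overlapping the box collision marks the machine available and enables player input; leaving it reverses both.
; Selection events store an item index, and accepting chains two map lookups, index to item to cost, printing the result only while available.
; No purchase or dispensing logic is present.
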(event OnComponentBeginOverlap(boxCol)
  (params (OverlappedComponent :type Primitive%20Component%20Object%20Reference) (OtherActor :type Actor%20Object%20Reference) (OtherComp :type Primitive%20Component%20Object%20Reference) (OtherBodyIndex :type Integer) (bFromSweep :type Boolean) (SweepResult :type Hit%20Result%20Structure%20%28by%20ref%29))
  (bind _output_get (Variables|Default|SetisVendingAvailable true))
  (Input|EnableInput (Game|GetPlayerController 0))
  (Development|PrintString "Hello"))

(event OnComponentEndOverlap(boxCol)
  (params (OverlappedComponent :type Primitive%20Component%20Object%20Reference) (OtherActor :type Actor%20Object%20Reference) (OtherComp :type Primitive%20Component%20Object%20Reference) (OtherBodyIndex :type Integer))
  (Variables|Default|SetisVendingAvailable false)
  (Input|DisableInput (Game|GetPlayerController 0)))

(event Custom|itemselected1
  (Variables|Default|Settestint 1))

(event Custom|itemselectred2
  (Variables|Default|Settestint 2))

(event Custom|itemselected3
  (Variables|Default|Settestint 3))

(event Custom|AcceptSelectedITem
  (CallFunction|Enter))

(event Custom|enter
  (if (stale OnComponentBeginOverlap(boxCol) _output_get)
    (bind _output_get (Variables|Default|Settestint (Variables|Default|Gettestint)))
    (Development|PrintString (.Value (Utilities|Map|Find (Variables|Default|GetcostNumb3r) (.Value (Utilities|Map|Find (Variables|Default|Getitemnumber) _output_get)))))))

(fn ConstructionScript)