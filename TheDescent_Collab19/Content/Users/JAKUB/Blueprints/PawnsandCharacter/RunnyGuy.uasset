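; RunnyGuy is an actor that slides its Man skeletal mesh to the position of its MoveToLocation component when play begins.
; The Movement timeline's Amp track drives a lerp from the mesh's current location each update, so the blend compounds rather than running from a fixed start.
; An unconnected node would ragdoll the mesh from the root bone, but it never runs.
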(event EventBeginPlay
  (Utilities|FlowControl|Sequence
    (:then_1
      (bind _amp (Timeline|Movement Play)
        (:Update
          (Transformation|SetWorldLocation (Variables|Default|GetMan) (Math|Vector|Lerp(Vector) (Transformation|GetWorldLocation (Variables|Default|GetMan)) (Transformation|GetWorldLocation (Variables|Default|GetMoveToLocation)) _amp) false false))))))

(fn ConstructionScript)