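; Game mode for the descent level that keeps a running player points total.
; Two events, addPointMyDude and takeAwayPoints, add or subtract a passed amount from PlayerPoints.
; Each change prints the new total with PrintString, with no clamping or other logic in the graph.
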(event Custom|addPointMyDude
  (params (points :type Integer))
  (bind _output_get (Variables|Default|SetplayerPoints (+ (Variables|Default|GetplayerPoints) points)))
  (Development|PrintString (Utilities|String|ToString(Integer) _output_get)))

(event Custom|takeAwayPoints
  (params (takeAwayPoint :type Integer))
  (bind _output_get (Variables|Default|SetplayerPoints (- (Variables|Default|GetplayerPoints) takeAwayPoint)))
  (Development|PrintString (Utilities|String|ToString(Integer) _output_get)))

(fn ConstructionScript)